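; BP_Mat1 is an actor whose water material changes colour with the player's distance from its plane.
; The construction script creates a dynamic material instance on the Plane mesh and stores it as WaterMat.
; Each tick maps the distance to the player pawn onto a clamped zero-to-one range up to MaxRange, then blends Col1 toward Col2 into the BaseColour parameter.
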(event EventTick
  (params (DeltaSeconds :type Float%20%28single-precision%29))
  ;[1 1 1] Set  colour
  (Rendering|Material|SetVectorParameterValue (Variables|Default|GetWaterMat) "BaseColour" (Math|Color|Lerp(LinearColor) (Variables|Default|GetCol1) (Variables|Default|GetCol2) (Math|Float|MapRangeClamped (Math|Vector|Distance(Vector) (Transformation|GetWorldLocation (Variables|Default|GetPlane)) (Transformation|GetActorLocation (Game|Player|GetPlayerPawn 0))) 0.0 (Variables|Default|GetMaxRange) 0.0 1.0)) :!class /Script/Engine.MaterialInstanceDynamic))

(fn ConstructionScript
  (bind _returnvalue (Rendering|Material|CreateDynamicMaterialInstance (Variables|Default|GetPlane) 0 "/Game/Materials/Material1.Material1" "None" :!class /Script/Engine.PrimitiveComponent))
  (Variables|Default|SetWaterMat _returnvalue))